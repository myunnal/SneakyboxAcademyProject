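; Game mode that runs a wave-based round system of spawned humans.
; On begin play it caches the first BP_HumanSpawner and starts the first round, with NextRound reading each round's spawn count from an array.
; HumansDied decrements the alive count and advances to the next round at zero.
; RestartRound resets the round index but passes a spawn count that evaluates to zero and leaves the alive count untouched.
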(event `self.ReceiveBeginPlay`
  (bind _outactors (`GameplayStatics.GetAllActorsOfClass` "/Game/Blueprints/BP_HumanSpawner.BP_HumanSpawner_C"))
  (set `self.HumanSpawnerRef` (`|GetArrayItem` _outactors))
  (`self.NextRound`))

(event `HumansDied`
  (set `self.AliveHumans` (- (`self.AliveHumans`) 1))
  (if (== (`self.AliveHumans`) 0)
    (`self.NextRound`)))

(fn `NextRound`
  (bind _output_get (set `self.HumansToSpawn` (`|GetArrayItem` (`self.RoundSpawnCount`) (`self.RoundNumber`))))
  (set `self.AliveHumans` _output_get)
  (`/Game/Blueprints/BP_HumanSpawner.StartSpawning` (`self.HumanSpawnerRef`) (`self.HumansToSpawn`))
  (set `self.RoundNumber` (+ (`self.RoundNumber`) 1)))

(fn `RestartRound`
  (set `self.RoundNumber` 0)
  (bind _output_get (set `self.HumansToSpawn` (+ 0 (* (`self.RoundNumber`) 0))))
  (bind _outactors (`GameplayStatics.GetAllActorsOfClass` "/Game/Blueprints/BP_HumanSpawner.BP_HumanSpawner_C"))
  (`/Game/Blueprints/BP_HumanSpawner.StartSpawning` (`|GetArrayItem` _outactors) _output_get))

(fn `UserConstructionScript`)